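; Test player controller that regenerates a FlatScape world from a given seed and noise intensity, then places the player on the new terrain.
; ResetWithSeed triggers generation, starts a short countdown and possesses a cached spectator pawn, or spawns one without possessing it.
; Tick runs the countdown, then queries ground height at the world origin and spawns or teleports a ThirdPersonCharacter just above it, then possesses it.
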(event `self.ReceiveTick`
  (params (DeltaSeconds :type "Float (single-precision)"))
  (`self.CheckReset` DeltaSeconds))

(fn `CheckReset`
  (params (deltaTime :type "Float (double-precision)"))
  (bind _createdpawn (`self.createdPawn`))
  (if (> (`self.resetTimer`) 0.0)
    (set `self.resetTimer` (- (`self.resetTimer`) deltaTime))
    (if (<= (`self.resetTimer`) 0.0)
      (bind _returnvalue (`GameplayStatics.GetActorOfClass` "/WorldScape/Blueprints/WorldScapeRoot/FlatScape.FlatScape_C"))
      (bind _returnvalue_2 (`WorldScapeRoot.GetGroundHeight` _returnvalue (`KismetMathLibrary.MakeVector` 0.0) false))
      (bind _returnvalue_3 (`KismetMathLibrary.MakeVector` 0.0 0.0 (+ _returnvalue_2 100.0)))
      (`SceneComponent.K2_SetWorldLocation` (`self.RootComponent`) _returnvalue_3 false true)
      (`/Engine/EditorBlueprintResources/StandardMacros.IsValid` _createdpawn
        (:`Is Valid`
          (`self.K2_SetActorLocation` _createdpawn _returnvalue_3 false true)
          (`self.Possess` _createdpawn))
        (:`Is Not Valid`
          (bind _returnvalue_4 (`|SpawnActorFromClass` "/Game/ThirdPersonBP/Blueprints/ThirdPersonCharacter.ThirdPersonCharacter_C" (`KismetMathLibrary.MakeTransform` _returnvalue_3) "AlwaysSpawn" "OverrideRootScale" null null))
          (`/Engine/EditorBlueprintResources/StandardMacros.IsValid` _returnvalue_4
            (:`Is Valid`
              (bind _output_get (set `self.createdPawn` _returnvalue_4))
              (`self.Possess` _output_get))))))))

(fn `ResetWithSeed`
  (params (Seed :type Integer) (Intensity :type Integer))
  (bind _spectator (`self.spectator`))
  (bind _returnvalue (`GameplayStatics.GetActorOfClass` "/WorldScape/Blueprints/WorldScapeRoot/FlatScape.FlatScape_C"))
  (`/Engine/EditorBlueprintResources/StandardMacros.IsValid` _returnvalue
    (:`Is Valid`
      (set `WorldScapeRoot.NoiseIntensity` (`KismetMathLibrary.Conv_IntToDouble` Intensity) _returnvalue)
      (set `WorldScapeRoot.Seed` Seed _returnvalue)
      (set `WorldScapeRoot.bGenerateWorldScape` true _returnvalue)
      (set `self.resetTimer` 2.0)
      (`/Engine/EditorBlueprintResources/StandardMacros.IsValid` _spectator
        (:`Is Valid`
          (`self.Possess` _spectator))
        (:`Is Not Valid`
          (bind _returnvalue_2 (`|SpawnActorFromClass` "/Script/Engine.SpectatorPawn" (`SceneComponent.K2_GetComponentToWorld` (`self.RootComponent`)) "Undefined" "OverrideRootScale" null null))
          (set `self.spectator` _returnvalue_2))))))

(fn `UserConstructionScript`
  (`parent.UserConstructionScript`))